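; BP_EnemyTarget is an enemy that detects pawns by sight and chases them when its attack state is on.
; PawnSensing triggers a one-time suspicion message on the seen pawn and, while attacking, an AI move toward it.
; Each sighting restarts a short retriggerable delay, so losing sight stops the message and re-arms it.
; StartAttack and StopAttack toggle the chase, with StopAttack redirecting the move to itself.
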(event OnSeePawn(PawnSensing)
  (params (Pawn :type Pawn%20Object%20Reference))
  (bind _self self)
  (Utilities|FlowControl|Sequence
    (:then_0
      (Utilities|FlowControl|Sequence
        (:then_0
          (Utilities|FlowControl|DoOnce false :!label _label
            (:Completed
              (Class|BPSuspicionInterface|StartSuspicion(Message) Pawn _self))))
        (:then_1
          (if (Variables|Default|GetAttack)
            (AI|AIMoveTo _self "0, 0, 0" Pawn 5.0 false)))))
    (:then_1
      (Utilities|FlowControl|RetriggerableDelay 1.0)
      (Class|BPSuspicionInterface|StopSuspicion(Message) Pawn)
      (goto _label Reset))))

(event EventStopAttack
  (bind _self self)
  (Variables|Default|SetAttack false)
  (AI|AIMoveTo _self "0, 0, 0" _self 5.0 false))

(event EventStartAttack
  (Variables|Default|SetAttack true))

(fn ConstructionScript)